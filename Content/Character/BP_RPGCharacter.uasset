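; RPG character Blueprint that handles keyboard toggles for the stat and quest UI.
; F adds or removes the widget held by StatWidgetComp from the viewport, while Q calls CreateQuestWidget or DestroyQuestWidget.
; Each toggle tracks its own visibility flag and switches the mouse cursor and input mode between Game And UI and Game Only, independently of the other.
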(event `Key|F`
  (params (Key :type "Key Structure"))
  (bind _returnvalue (`GameplayStatics.GetPlayerController` 0))
  (bind _returnvalue_2 (`GameplayStatics.GetPlayerController` 0))
  (bind _returnvalue_3 (`WidgetComponent.GetWidget` (`self.StatWidgetComp`)))
  ;[1 1 1] Stat Widget
  (:`Pressed`
    (if (`self.ShowingStatWidget`)
      (`Widget.RemoveFromParent` _returnvalue_3)
      (set `PlayerController.bShowMouseCursor` false _returnvalue)
      (set `self.ShowingStatWidget` false)
      (`WidgetBlueprintLibrary.SetInputMode_GameOnly` _returnvalue)
      (else
        (`UserWidget.AddToViewport` _returnvalue_3 0)
        (set `PlayerController.bShowMouseCursor` true _returnvalue_2)
        (set `self.ShowingStatWidget` true)
        (`WidgetBlueprintLibrary.SetInputMode_GameAndUIEx` _returnvalue_2 _returnvalue_3 "DoNotLock" true true)))))

(event `Key|Q`
  (params (Key :type "Key Structure"))
  (bind _returnvalue (`GameplayStatics.GetPlayerController` 0))
  (bind _returnvalue_2 (`GameplayStatics.GetPlayerController` 0))
  (:`Pressed`
    (if (not (`self.ShowingQusetWidget`))
      (`self.CreateQuestWidget`)
      (set `self.ShowingQusetWidget` true)
      (set `PlayerController.bShowMouseCursor` true _returnvalue)
      (`WidgetBlueprintLibrary.SetInputMode_GameAndUIEx` _returnvalue null "DoNotLock" true true)
      (else
        (`self.DestroyQuestWidget`)
        (set `self.ShowingQusetWidget` false)
        (set `PlayerController.bShowMouseCursor` false _returnvalue_2)
        (`WidgetBlueprintLibrary.SetInputMode_GameOnly` _returnvalue_2)))))

(fn `UserConstructionScript`)